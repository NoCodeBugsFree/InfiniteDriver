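; Game mode for a truck driving game that handles the menu-to-player camera switch, save data, leaderboards and achievements.
; BeginPlay shows the menu camera, loads or creates the SharkSave slot, then pulls a higher online best distance into it and caches achievements.
; Retry events save high scores with a retry flag.
; Round end records new bests, posts distance and writes achievement progress from cars crashed and coins against per-achievement targets.
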(event Custom|Update%20LeaderBoards%20at%20round%20end
  ;[1 1 1] Save Scores again?
  (bind _astruck_vehicle (Utilities|Casting|CastToTruckVehicle (Game|Player|GetPlayerPawn 0)))
  (Variables|Default|SetCurrentDistanceRef (Variables|/Game/Blueprints/TruckVehicle.TruckVehicle_C|GetCurrentDistance _astruck_vehicle))
  (bind _output_get (Variables|Default|SetCurrentCoinsRef (Variables|/Game/Blueprints/TruckVehicle.TruckVehicle_C|GetCollectedCoins _astruck_vehicle)))
  (if (> _output_get (Variables|Default|GetHighScoreCoinsRef))
    (bind _asshark_save (Utilities|Casting|CastToSharkSave (Variables|Default|GetSaveGameRef)))
    (Variables|/Game/Blueprints/SharkSave.SharkSave_C|SetHighScoreCoins _asshark_save (Variables|Default|GetCurrentCoinsRef)))
  (if (> (Variables|Default|GetCurrentDistanceRef) (Variables|Default|GetHighScoreDistanceRef))
    (bind _asshark_save_2 (Utilities|Casting|CastToSharkSave (Variables|Default|GetSaveGameRef)))
    (Variables|/Game/Blueprints/SharkSave.SharkSave_C|SetHighScoreDistance _asshark_save_2 (Variables|Default|GetCurrentDistanceRef))
    (SaveGame|SaveGametoSlot _asshark_save_2 "Slot1")
    ;[1 1 1] Write leaderboard and save again
    (Class|LeaderboardBlueprintLibrary|WriteLeaderboardInteger (Game|GetPlayerController 0) "best_distance" (Variables|Default|GetCurrentDistanceRef)))
  (CallFunction|CheckAchievementsEvent))

(event Custom|Save%20If%20retry%20level
  ;[1 1 1] Retry Level
  (bind _returnvalue (SaveGame|DoesSaveGameExist "Slot1"))
  (if _returnvalue
    (bind _astruck_vehicle (Utilities|Casting|CastToTruckVehicle (Game|Player|GetPlayerPawn 0)))
    (bind _asshark_save (Utilities|Casting|CastToSharkSave (Variables|Default|GetSaveGameRef)))
    (Variables|/Game/Blueprints/SharkSave.SharkSave_C|SetRetryLevel _asshark_save true)
    (Variables|/Game/Blueprints/SharkSave.SharkSave_C|SetHighScoreDistance _asshark_save (Variables|/Game/Blueprints/TruckVehicle.TruckVehicle_C|GetHighScoreDistanceRef _astruck_vehicle))
    (Variables|/Game/Blueprints/SharkSave.SharkSave_C|SetHighScoreCoins _asshark_save (Variables|/Game/Blueprints/TruckVehicle.TruckVehicle_C|GetHighScoreCoinRef _astruck_vehicle))
    (SaveGame|SaveGametoSlot _asshark_save "Slot1")))

(event Custom|Not%20retry%20level
  ;[1 1 1] Reset Retry Level
  (bind _returnvalue (SaveGame|DoesSaveGameExist "Slot1"))
  (if _returnvalue
    (bind _astruck_vehicle (Utilities|Casting|CastToTruckVehicle (Game|Player|GetPlayerPawn 0)))
    (bind _asshark_save (Utilities|Casting|CastToSharkSave (Variables|Default|GetSaveGameRef)))
    (Variables|/Game/Blueprints/SharkSave.SharkSave_C|SetRetryLevel _asshark_save false)
    (Variables|/Game/Blueprints/SharkSave.SharkSave_C|SetHighScoreDistance _asshark_save (Variables|/Game/Blueprints/TruckVehicle.TruckVehicle_C|GetHighScoreDistanceRef _astruck_vehicle))
    (Variables|/Game/Blueprints/SharkSave.SharkSave_C|SetHighScoreCoins _asshark_save (Variables|/Game/Blueprints/TruckVehicle.TruckVehicle_C|GetHighScoreCoinRef _astruck_vehicle))
    (SaveGame|SaveGametoSlot _asshark_save "Slot1")))

(event Custom|CheckLeaderBoards
  ;[0 0.1091 1] Check if played on other device
  (bind _leaderboardvalue (|LeaderboardQuery (Game|GetPlayerController 0) "best_distance")
    (:OnSuccess
      (if (> _leaderboardvalue (Variables|Default|GetHighScoreDistanceRef))
        (bind _output_get (Variables|Default|SetHighScoreDistanceRef _leaderboardvalue))
        (bind _asshark_save (Utilities|Casting|CastToSharkSave (Variables|Default|GetSaveGameRef)))
        (Variables|/Game/Blueprints/SharkSave.SharkSave_C|SetHighScoreDistance _asshark_save _output_get)
        (SaveGame|SaveGametoSlot _asshark_save "Slot1"))
      (CallFunction|UpdateAchievements))))

(event Custom|Update%20Achievements
  ;[1 1 1] Cache n update
  (Class|LeaderboardBlueprintLibrary|WriteLeaderboardInteger (Game|GetPlayerController 0) "best_distance" (Variables|Default|GetHighScoreDistanceRef))
  (|CacheAchievements (Game|GetPlayerController 0)))

(event Custom|Write%20Achievements
  (params (AchievementName :type Name) (Percent :type Float%20%28single-precision%29) (Index :type Integer))
  ;[1 0.5763 0] Write Achievments
  (bind (_writtenachievementname _writtenprogress _writtenusertag) (|WriteAchievementProgress (Game|GetPlayerController 0) AchievementName Percent Index)
    (:OnSuccess
      (bind _asshark_save (Utilities|Casting|CastToSharkSave (Variables|Default|GetSaveGameRef)))
      (Utilities|Array|SetArrayElem (Variables|/Game/Blueprints/SharkSave.SharkSave_C|GetWrittenAchievements _asshark_save) _writtenusertag _writtenprogress)
      (SaveGame|SaveGametoSlot _asshark_save "Slot1"))))

(event Custom|Check%20Achievements%20Event
  ;[0 0.8245 1] Check and save achievements
  (bind _astruck_vehicle (Utilities|Casting|CastToTruckVehicle (Game|Player|GetPlayerPawn 0)))
  (CallFunction|CheckAchievements (Variables|/Game/Blueprints/TruckVehicle.TruckVehicle_C|GetCrasCrahed _astruck_vehicle) 3 4) ; Distance Achievements
  (CallFunction|CheckAchievements (Variables|/Game/Blueprints/TruckVehicle.TruckVehicle_C|GetCollectedCoins _astruck_vehicle) 0 2) ; Distance Achievements
  (bind _asshark_save (Utilities|Casting|CastToSharkSave (Variables|Default|GetSaveGameRef)))
  (Variables|/Game/Blueprints/SharkSave.SharkSave_C|SetAchievementProgress _asshark_save (Variables|Default|GetAchievementProgress))
  (SaveGame|SaveGametoSlot _asshark_save "Slot1"))

(event EventBeginPlay
  ;[0 0.1091 1] Main Menu Cam
  (if (not (Variables|Default|GetGameHasStarted))
    (bind _outactors (Actor|GetAllActorsOfClass "/Game/Blueprints/MatrixCam1.MatrixCam1_C"))
    (Game|Player|SetViewTargetwithBlend (Game|GetPlayerController 0) (Utilities|Array|Get(acopy) _outactors) 0.0 "VTBlend_Linear" 0.0 false)
    ;[0 0.8245 1] Save Game Data Tasks
    (bind _returnvalue (SaveGame|DoesSaveGameExist "Slot1"))
    (if _returnvalue
      (bind _returnvalue_2 (SaveGame|LoadGamefromSlot "Slot1"))
      (bind _asshark_save (Utilities|Casting|CastToSharkSave _returnvalue_2))
      (Variables|Default|SetSaveGameRef _asshark_save)
      (Variables|Default|SetRetry (Variables|/Game/Blueprints/SharkSave.SharkSave_C|GetRetryLevel _asshark_save))
      (else
        (bind _returnvalue_3 (SaveGame|CreateSaveGameObject "/Game/Blueprints/SharkSave.SharkSave_C"))
        (bind _output_get (Variables|Default|SetSaveGameRef _returnvalue_3))
        (bind _asshark_save_2 (Utilities|Casting|CastToSharkSave _output_get))
        (Variables|/Game/Blueprints/SharkSave.SharkSave_C|SetRetryLevel _asshark_save_2 false)
        (Variables|/Game/Blueprints/SharkSave.SharkSave_C|SetHighScoreCoins _asshark_save_2 0)
        (Variables|/Game/Blueprints/SharkSave.SharkSave_C|SetHighScoreDistance _asshark_save_2 0)
        (SaveGame|SaveGametoSlot _asshark_save_2 "Slot1")))
    ;[1 1 1] Set Reference Variables
    (bind _asshark_save_3 (Utilities|Casting|CastToSharkSave (Variables|Default|GetSaveGameRef)))
    (Variables|Default|SetHighScoreDistanceRef (Variables|/Game/Blueprints/SharkSave.SharkSave_C|GetHighScoreDistance _asshark_save_3))
    (Variables|Default|SetHighScoreCoinsRef (Variables|/Game/Blueprints/SharkSave.SharkSave_C|GetHighScoreCoins _asshark_save_3))
    (CallFunction|CheckLeaderBoards)))

(event EventStartedEvent
  (params (Started :type Boolean))
  ;[1 1 1] On start go to player cam
  (bind _output_get (Variables|Default|SetGameHasStarted Started))
  (if _output_get
    (Game|Player|SetViewTargetwithBlend (Game|GetPlayerController 0) (Game|Player|GetPlayerPawn 0) 0.5 "VTBlend_Linear" 0.0 false)))

(fn ConstructionScript)

(fn CheckAchievements
  (params (Start%20to%20Check :type Integer) (Start%20Index :type Integer) (EndIndex :type Integer))
  (for _index (range Start%20Index EndIndex) ; Check AchievementValues Array
    (bind (_bfoundid _progress) (Class|AchievementBlueprintLibrary|GetCachedAchievementProgress (Game|GetPlayerController 0) (Utilities|Array|Get(acopy) (Variables|Default|GetAchievementNames) _index)))
    (if _bfoundid
      (if (> (Math|Float|Clamp(Float) (* (/ (Math|Conversions|ToFloat(Integer) Start%20to%20Check) (Math|Conversions|ToFloat(Integer) (Utilities|Array|Get(acopy) (Variables|Default|GetAchievementValues) _index))) 1e+02) 0.0 1e+02) _progress) ; Current Value higher than Game Center
        (CallFunction|WriteAchievements (Utilities|Array|Get(acopy) (Variables|Default|GetAchievementNames) _index) (Math|Float|Clamp(Float) (* (/ (Math|Conversions|ToFloat(Integer) Start%20to%20Check) (Math|Conversions|ToFloat(Integer) (Utilities|Array|Get(acopy) (Variables|Default|GetAchievementValues) _index))) 1e+02) 0.0 1e+02) _index :!label _label)
        (else
          (Utilities|Array|SetArrayElem (Variables|Default|GetAchievementProgress) _index _progress)
          (bind _asshark_save (Utilities|Casting|CastToSharkSave (Variables|Default|GetSaveGameRef)))
          (Utilities|Array|SetArrayElem (Variables|/Game/Blueprints/SharkSave.SharkSave_C|GetWrittenAchievements _asshark_save) _index _progress)))
      (else
        (bind _asshark_save_2 (Utilities|Casting|CastToSharkSave (Variables|Default|GetSaveGameRef)))
        (if (>= (Utilities|Array|Get(acopy) (Variables|Default|GetAchievementProgress) _index) (Utilities|Array|Get(acopy) (Variables|/Game/Blueprints/SharkSave.SharkSave_C|GetAchievementProgress _asshark_save_2) _index)) ; Progress is greater than last reported
          (goto _label))))))

(fn CoinsCollected
  (return 0))

(fn DamageTaken
  (return 0.0))

(fn DistanceTravel
  (return ""))