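; CoinBP is a collectible coin that spins and is picked up by the player.
; On BeginPlay a timeline's updates rotate the coin and its shadow in yaw at a randomized per-update speed.
; Overlaps are matched by component name: "Overlapper" plays a sound, notifies the player pawn and destroys the coin, while "Sweeper" purges it silently.
; A DelDistance graph holds an unused distance-behind-player check.
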(event OnComponentBeginOverlap(Coin)
  (params (OverlappedComponent :type Primitive%20Component%20Object%20Reference) (OtherActor :type Actor%20Object%20Reference) (OtherComp :type Primitive%20Component%20Object%20Reference) (OtherBodyIndex :type Integer) (bFromSweep :type Boolean) (SweepResult :type Hit%20Result%20Structure%20%28by%20ref%29))
  (bind _returnvalue (Utilities|String|ToString(Object) OtherComp))
  ;[1 1 1] Coin Collected
  (if (Utilities|Enum|Equal(Enum) _returnvalue "Overlapper")
    (Audio|PlaySoundatLocation 0 (Transformation|GetActorLocation))
    (Class|BPInterface|CoinsCollectedExec(Message) (Game|Player|GetPlayerPawn 0))
    (Actor|DestroyActor)
    (else
      ;[1 1 1] Purge
      (if (Utilities|Enum|Equal(Enum) _returnvalue "Sweeper")
        (Actor|DestroyActor)))))

(event EventBeginPlay
  ;[1 1 1] Animate Coin
  (Variables|Default|SetRotSpeed (Math|Random|RandomFloatinRange 0.8 1.2))
  (Timeline|Timeline_0 Play
    (:Update
      (Transformation|AddRelativeRotation (Variables|Default|GetCoin) (Math|Rotator|MakeRotator 0.0 0.0 (Variables|Default|GetRotSpeed)) false true))))

(fn ConstructionScript)