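; Endless-road track segment for a truck driving game that recycles itself and randomises its scenery, traffic and pickups.
; On BeginPlay it randomly shows a bridge that crashes the truck on hit, then scatters trees at tagged billboards and coins around itself.
; Segments spawned at runtime place three sedans at shuffled spawn points, with direction set from rotation.
; When the truck's Sweeper leaves far enough ahead, it spawns a segment further forward and destroys itself.
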(event OnComponentEndOverlap(Ground)
  (params (OverlappedComponent :type Primitive%20Component%20Object%20Reference) (OtherActor :type Actor%20Object%20Reference) (OtherComp :type Primitive%20Component%20Object%20Reference) (OtherBodyIndex :type Integer))
  ;[1 1 1] Sweeper Detected
  (Utilities|Casting|CastToTruckVehicle OtherActor)
  (if (Utilities|Enum|Equal(Enum) (Utilities|String|ToString(Object) OtherComp) "Sweeper")
    (Utilities|DeletionDistance
      (:out
        ;[1 1 1] Spawn New segment
        (bind _returnvalue (Game|SpawnActorfromClass "TrackSpawn_C" (Utilities|Skip2TracksLocation) "AdjustIfPossibleButDontSpawnIfColliding" 0 (Game|Player|GetPlayerPawn 0)))
        (Variables|TrackSpawn_C|SetWasSpawned _returnvalue true)
        ;[1 1 1] Destroy self
        (Actor|DestroyActor)))))

(event OnComponentHit(BridgeMid)
  (params (HitComponent :type Primitive%20Component%20Object%20Reference) (OtherActor :type Actor%20Object%20Reference) (OtherComp :type Primitive%20Component%20Object%20Reference) (NormalImpulse :type Vector :default "0, 0, 0") (Hit :type Hit%20Result%20Structure%20%28by%20ref%29))
  ;[1 1 1] Truck Hit Bridge
  (if (Utilities|Enum|Equal(Enum) (Utilities|String|ToString(Object) OtherComp) "VehicleMesh")
    (bind _astruck_vehicle (Utilities|Casting|CastToTruckVehicle OtherActor))
    (Variables|/Game/Blueprints/TruckVehicle.TruckVehicle_C|SetCrashed _astruck_vehicle true)))

(event Custom|RandomSpawn
  (bind _spawnlocations (Variables|Default|GetSpawnLocations))
  ;[1 1 1] Spawn Cars at random points
  (Utilities|Array|Shuffle _spawnlocations)
  (for _index (range 0 2) ; Spawn 3 Cars
    (bind _returnvalue (Game|SpawnActorfromClass "/Game/Blueprints/SedanBP.SedanBP_C" (Utilities|Array|Get(acopy) _spawnlocations _index) "AlwaysSpawn" 0 (Game|Player|GetPlayerPawn 0)))
    (bind _assedan_bp (Utilities|Casting|CastToSedanBP _returnvalue))
    (if (Utilities|CheckDirectionSpawned (Transformation|GetWorldRotation _returnvalue))
      (Variables|/Game/Blueprints/SedanBP.SedanBP_C|SetDrivingFwd _assedan_bp false)
      (else
        (Variables|/Game/Blueprints/SedanBP.SedanBP_C|SetDrivingFwd _assedan_bp true)))))

(event EventTick
  (params (DeltaSeconds :type Float%20%28single-precision%29))
  ;[1 1 1] Tick Event
  ;[1 1 1] Add spawn Points to Array
  (if (Variables|Default|GetWasSpawned)
    (Utilities|FlowControl|DoOnce false
      (:Completed
        (for _array_element (Actor|GetComponentsbyTag "/Script/Engine.BillboardComponent" "SpawnPoint")
          (Utilities|Array|AddUnique (Variables|Default|GetSpawnLocations) (Transformation|GetWorldTransform _array_element)))
        (CallFunction|RandomSpawn)))))

(event EventBeginPlay
  ;[0 0.1091 1] Random Spawning
  (if (== (Math|Random|RandomIntegerinRange 1 4) 2)
    (Utilities|ShowBridge
      (:NewParam
        _))
    (else
      (Utilities|HideBridge
        (:NewParam
          _))))
  (|RandomTreeSPawn
    (:NewParam
      ;[1 1 1] Coin Spawning
      (Utilities|FlowControl|Delay 0.05)
      (for _index (range 1 2)
        (Game|SpawnActorfromClass "/Game/Blueprints/CoinBP.CoinBP_C" (Utilities|CoinSpawnTransform (Transformation|GetWorldLocation)) "AdjustIfPossibleButDontSpawnIfColliding" 0 0))
      (for _index_2 (range 1 2)
        (Game|SpawnActorfromClass "/Game/Blueprints/CoinBP.CoinBP_C" (Utilities|CoinSpawnTransform (Transformation|GetWorldLocation)) "AdjustIfPossibleButDontSpawnIfColliding" 0 0))
      (for _index_3 (range 1 2)
        (Game|SpawnActorfromClass "/Game/Blueprints/CoinBP.CoinBP_C" (Utilities|CoinSpawnTransform (Transformation|GetWorldLocation)) "AdjustIfPossibleButDontSpawnIfColliding" 0 0)))))

(fn ConstructionScript)