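; Player truck for an endless lane-changing road runner that drives forward automatically once the game starts.
; Lane changes spawn a LaneChanger target ahead, which steering follows until overlapped, otherwise aiming at TrackSpawn lane points.
; Tick also tracks distance against the loaded high score, spawns repair kits and random power-ups, applies rocket boost and moves the camera.
; Car hits drain health unless boosted; crashing stops the truck, slows time, switches camera and shows game over.
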(event Custom|SaveScores
  (bind _collectedcoins (Variables|Default|GetCollectedCoins))
  ;[0 0.8245 1] Set Save Distance HighScore
  (Utilities|FlowControl|DoOnce false
    (:Completed
      (if (> (stale EventTick _distance) (Variables|Default|GetHighScoreDistanceRef))
        (Variables|Default|SetHighScoreDistanceRef (stale EventTick _distance))
        (elif (> _collectedcoins (Variables|Default|GetHighScoreCoinRef))
          (Variables|Default|SetHighScoreCoinRef _collectedcoins))))))

(event Custom|ResetTask
  (bind _collectedcoins (Variables|Default|GetCollectedCoins))
  ;[0 0.8245 1] Set Save Distance HighScore
  (Utilities|FlowControl|DoOnce false) ; enters at Reset
)

(event EventStartedEvent
  (params (Started :type Boolean))
  ;[1 0 0.9041] Interface Events
  (Variables|Default|SetGameHasStarted Started))

(event EventTick
  (params (DeltaSeconds :type Float%20%28single-precision%29))
  ;[1 0 0] Tick Event
  (if (Variables|Default|GetGameHasStarted)
    (Utilities|FlowControl|Sequence
      (:then_0
        ;[1 0.3949 0] Checks
        (if (not (Variables|Default|GetCrashed))
          (|MovementLogic :!label _label)
          (else
            (|CrashEndGameLogic
              (:Out
                (CallFunction|SaveScores)
                (CallFunction|GameOver))))))
      (:then_1
        (goto _label HandBrake%20Input))
      (:then_2
        (bind _distance (Utilities|DistanceTravelled)
          (:out
            ;[1 1 1] Spawn New HighScore Widget
            (Utilities|NewHighScoreMacro (> _distance (Variables|Default|GetHighScoreDistanceRef))))))
      (:then_3
        (|RepairKitSpawning))
      (:then_4
        (|RocketPowerUp))
      (:then_5
        (|SetCameraPosition)))
    (else
      ;[1 1 1] Keep Truck Still on Menu Screen
      (Transformation|SetActorLocation (Variables|Default|GetStartLocation) false true))))

(event EventBeginPlay
  ;[0 0.1091 1] Begin Play
  (CallFunction|ResetTask)
  (Class|PlayerController|SetAudioListenerOverride (Game|GetPlayerController 0) (Variables|Default|GetDriver) "0, 0, 0" "0, 0, 0")
  (Variables|Default|SetStartLocation (Transformation|GetActorLocation))
  (Rendering|SetVisibility (Variables|Default|Getflamepower) false false)
  (Audio|SpawnSoundAttached 0 (Variables|Character|GetMesh) "None" (Transformation|GetActorLocation))
  (bind _returnvalue (Audio|SpawnSoundAttached 0 (Variables|Default|GetDriver) "None" "0, 0, 0" "0, 0, 0" "SnapToTarget" true 0.75))
  (Variables|Default|SetTruckIdleSound _returnvalue)
  ;[0 0.8245 1] Get Save Game Reference Data
  (Utilities|FlowControl|Delay 0.05)
  (bind _returnvalue_2 (SaveGame|DoesSaveGameExist "Slot1"))
  (if _returnvalue_2
    (bind _returnvalue_3 (SaveGame|LoadGamefromSlot "Slot1"))
    (bind _output_get (Variables|Default|SetSaveRef _returnvalue_3))
    (bind _asshark_save (Utilities|Casting|CastToSharkSave _output_get))
    (Variables|Default|SetHighScoreCoinRef (Variables|/Game/Blueprints/SharkSave.SharkSave_C|GetHighScoreCoins _asshark_save))
    (Variables|Default|SetHighScoreDistanceRef (Variables|/Game/Blueprints/SharkSave.SharkSave_C|GetHighScoreDistance _asshark_save))))

(event EventCoinsCollectedExec
  ;[1 0 0.9041] Interface Events
  (Variables|Default|SetCollectedCoins (+ (Variables|Default|GetCollectedCoins) 1)))

(fn ConstructionScript)

(fn GameOver
  (bind _assharksporter_hud (Utilities|Casting|CastToSharksporterHUD (HUD|GetHUD (Game|GetPlayerController 0))))
  (Default|GameOver (Variables|/Game/HUD/SharksporterHUD.SharksporterHUD_C|GetWidgetHUD _assharksporter_hud)))

(fn CoinsCollected
  (return (Variables|Default|GetCollectedCoins)))

(fn DamageTaken
  (return (Variables|Default|GetDamageTakenVar)))

(fn DistanceTravel
  (return (Variables|Default|GetDistanceCheck)))

(event Custom|RocketAnabled
  (bind _flamepower (Variables|Default|Getflamepower))
  (Variables|Default|SetPoweredUp true)
  (Rendering|SetVisibility _flamepower true false)
  (Utilities|FlowControl|Delay 3.0)
  (Variables|Default|SetPoweredUp false)
  (Rendering|SetVisibility _flamepower false false))

(event OnComponentBeginOverlap(Overlapper)
  (params (OverlappedComponent :type Primitive%20Component%20Object%20Reference) (OtherActor :type Actor%20Object%20Reference) (OtherComp :type Primitive%20Component%20Object%20Reference) (OtherBodyIndex :type Integer) (bFromSweep :type Boolean) (SweepResult :type Hit%20Result%20Structure%20%28by%20ref%29))
  (bind _returnvalue (Utilities|String|ToString(Object) OtherComp))
  ;[1 0.9449 0.01816] SelectLane
  (bind _astrack_spawn (Utilities|Casting|CastToTrackSpawn OtherActor)
    (:then
      (if (Utilities|Enum|Equal(Enum) _returnvalue "LeftLane")
        (Variables|Default|SetIsInLeftLane true)
        (Variables|Default|SetFwdVector (Utilities|StraightAheadVector _astrack_spawn _astrack_spawn) :!label _label)
        (Variables|Default|SetIsInFarRightLane false)
        (Variables|Default|SetIsInFarLeftLane false)
        (elif (Utilities|Enum|Equal(Enum) _returnvalue "RightLane")
          (Variables|Default|SetIsInLeftLane false)
          (goto _label)
          (elif (Utilities|Enum|Equal(Enum) _returnvalue "FarLeftLane")
            (Variables|Default|SetIsInFarLeftLane true)
            (Variables|Default|SetIsInFarRightLane false)
            (Variables|Default|SetFwdVector (Utilities|StraightAheadVectorFar _astrack_spawn _astrack_spawn) :!label _label_2)
            (elif (Utilities|Enum|Equal(Enum) _returnvalue "FarRightLane")
              (Variables|Default|SetIsInFarLeftLane false)
              (Variables|Default|SetIsInFarRightLane true)
              (goto _label_2))))))
    (:CastFailed
      ;[1 1 1] If Turn Target reached, delete target
      (bind _aslane_changer (Utilities|Casting|CastToLaneChanger OtherActor))
      (Variables|Default|SetIsTurning false)
      (Actor|DestroyActor _aslane_changer))))

(event Custom|FireChangeLeft
  ;[1 1 1] Turn Left
  (if (not (or (Variables|Default|GetIsTurning) (Variables|Default|GetIsInFarLeftLane)))
    (Variables|Default|SetTurningLeft true)
    ;[1 1 1] Creates overlapping helper. This checks if Turn has been reached
    (bind _returnvalue (Game|SpawnActorfromClass "/Game/Blueprints/LaneChanger.LaneChanger_C" (Math|Transform|MakeTransform (Utilities|TurningDirection)) "AdjustIfPossibleButDontSpawnIfColliding" 0 self))
    (Variables|Default|SetNewTurn _returnvalue)
    (Variables|Default|SetNewTurnVector (Transformation|GetWorldLocation (Variables|Default|GetNewTurn)))
    (Variables|Default|SetIsTurning true)
    (Audio|SpawnSoundAttached 0 (Variables|Default|GetDriver) "None" "0, 0, 0" "0, 0, 0" "SnapToTarget" true)))

(event Custom|FireChangeRight
  ;[1 1 1] Turn Right
  (if (not (or (Variables|Default|GetIsTurning) (Variables|Default|GetIsInFarRightLane)))
    (Variables|Default|SetTurningLeft false)
    ;[1 1 1] Creates overlapping helper. This checks if Turn has been reached
    (bind _returnvalue (Game|SpawnActorfromClass "/Game/Blueprints/LaneChanger.LaneChanger_C" (Math|Transform|MakeTransform (Utilities|TurningDirection)) "AdjustIfPossibleButDontSpawnIfColliding" 0 self))
    (Variables|Default|SetNewTurn _returnvalue)
    (Variables|Default|SetNewTurnVector (Transformation|GetWorldLocation (Variables|Default|GetNewTurn)))
    (Variables|Default|SetIsTurning true)
    (Audio|SpawnSoundAttached 0 (Variables|Default|GetDriver) "None" "0, 0, 0" "0, 0, 0" "SnapToTarget" true)))

(event OnComponentHit(Overlapper)
  (params (HitComponent :type Primitive%20Component%20Object%20Reference) (OtherActor :type Actor%20Object%20Reference) (OtherComp :type Primitive%20Component%20Object%20Reference) (NormalImpulse :type Vector :default "0, 0, 0") (Hit :type Hit%20Result%20Structure%20%28by%20ref%29))
  ;[1 1 1] Hits a car
  (bind _assedan_bp (Utilities|Casting|CastToSedanBP OtherActor))
  (CallFunction|ControlwhenCrashed)
  (Default|StruckbyTruck _assedan_bp)
  (Utilities|FlowControl|Delay 0.2)
  (if (not (Variables|Default|GetPoweredUp))
    (Utilities|SubstractDamage)))

(event Custom|Control%20When%20crashed
  ;[1 1 1] Check if crashing
  (if (<= (Variables|Default|GetDamageTakenVar) 0.0)
    (Variables|Default|SetCrashed true)))

(event Custom|AddHp
  ;[1 1 1] Increase Health
  (Utilities|AddDamage))