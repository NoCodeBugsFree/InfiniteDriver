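; Repair kit pickup that restores health to a TruckVehicle that overlaps it.
; A timeline started on BeginPlay spins the mesh and a separate Shadow component by small local rotation steps, each on its own axis.
; On overlap with a truck it calls AddHp, plays a sound, shows a RepairUMG widget given the pickup's world location, then destroys itself.
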(event EventBeginPlay
  ;[1 1 1] Set rotation
  (Timeline|TurnLoop Play
    (:Update
      (Transformation|AddLocalRotation (Variables|Default|GetStaticMesh) "0, 0,1.000000" false false)
      (Transformation|AddLocalRotation (Variables|Default|GetShadow) "0.000000,1.000000,0.000000" false false))))

(event Collision|EventActorBeginOverlap
  (params (OtherActor :type Actor%20Object%20Reference))
  (bind _astruck_vehicle (Utilities|Casting|CastToTruckVehicle OtherActor))
  (Default|AddHp _astruck_vehicle)
  (Audio|PlaySoundatLocation 0 (Transformation|GetActorLocation))
  (bind _returnvalue (UserInterface|CreateWidget "/Game/HUD/RepairUMG.RepairUMG_C"))
  (Variables|/Game/HUD/RepairUMG.RepairUMG_C|SetWorldLocation _returnvalue (Transformation|GetActorLocation))
  (UserInterface|Viewport|AddtoViewport _returnvalue 0)
  (Actor|DestroyActor))

(fn ConstructionScript)