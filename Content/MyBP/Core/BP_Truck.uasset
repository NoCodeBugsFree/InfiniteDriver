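; BP_Truck is the vehicle Blueprint for a truck, handling on-screen pickup-style messages and the game-over sequence.
; SpawnScreenFX adds a WBP_FXWidget to the viewport, its text chosen by message type.
; GameOver, also bound to debug key G, halts the truck, slows global time, blends to a camera spawned at GameoverCameraLocation and shakes it.
; It then quits after a Delay, which runs in the slowed game time.
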(event EventSpawnScreenFX
  (params (MessageType :type EMessageType%20Enum :default "MT_POOF"))
  ;[1 1 1] Poof
  (bind _returnvalue (UserInterface|CreateWidget "/Game/MyBP/UI/WBP_FXWidget.WBP_FXWidget_C"))
  (Rendering|Components|TextRender|SetText (Variables|/Script/InfiniteDriver.FXWidget|GetMessage _returnvalue) (Utilities|Select :Index MessageType :MT_POOF "POOF" :MT_COIN "COIN" :MT_REPAIR "REPAIR" :MT_POWERUP "POWER"))
  (UserInterface|Viewport|AddtoViewport _returnvalue 0))

(event EventGameOver
  (bind _returnvalue (Pawn|GetController))
  (bind _vehiclemovement (Variables|Default|GetVehicleMovement))
  (bind _asplayer_controller (Utilities|Casting|CastToPlayerController _returnvalue))
  ;[0 0.07145 1] Game Over
  (Components|Movement|StopMovementImmediately _vehiclemovement)
  (Class|WheeledVehicleMovementComponent|SetHandbrakeInput _vehiclemovement true)
  (Utilities|Time|SetGlobalTimeDilation 0.01)
  (bind _returnvalue_2 (Game|SpawnActorfromClass "/Script/Engine.CameraActor" (Transformation|GetWorldTransform (Variables|Default|GetGameoverCameraLocation)) "AlwaysSpawn" 0 0))
  (Game|Player|SetViewTargetwithBlend _asplayer_controller _returnvalue_2 0.0 "VTBlend_Linear" 0.0 false)
  (Class|PlayerController|ClientPlayCameraShake _asplayer_controller "/Game/MyBP/Other/BP_GameOverCameraShake.BP_GameOverCameraShake_C" 1.0 "CameraLocal" "0, 0, 0")
  (Utilities|FlowControl|Delay 5.0)
  (Game|QuitGame 0 "Quit"))

(event Input|KeyboardEvents|G
  (params (Key :type Key%20Structure))
  ;[1 0 0] DEBUG
  (:Pressed
    (Class|Truck|GameOver)))

(fn ConstructionScript)