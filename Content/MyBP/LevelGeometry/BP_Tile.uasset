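; BP_Tile is a level tile that spawns sedans on its lanes and random pickups inside a volume.
; BeginPlay gathers four lane components, and SpawnCars places a BP_Sedan at each lane's world transform.
; SpawnPickups picks a random class from Pickups and spawns it enlarged at a random point, printing an error if the list is empty.
; Overlapping BridgeM destroys sedans, while a truck game-over branch is an unconnected TODO.
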(event OnComponentBeginOverlap(BridgeM)
  (params (OverlappedComponent :type Primitive%20Component%20Object%20Reference) (OtherActor :type Actor%20Object%20Reference) (OtherComp :type Primitive%20Component%20Object%20Reference) (OtherBodyIndex :type Integer) (bFromSweep :type Boolean) (SweepResult :type Hit%20Result%20Structure%20%28by%20ref%29))
  (Utilities|FlowControl|Sequence
    (:then_0
      (bind _asbp_sedan (Utilities|Casting|CastToBP_Sedan OtherActor))
      (Actor|DestroyActor _asbp_sedan))))

(event EventBeginPlay
  (Variables|Default|SetLanes (Utilities|Array|MakeArray (Variables|Default|GetLane02) (Variables|Default|GetLane03) (Variables|Default|GetLane01) (Variables|Default|GetLane04))))

(event EventSpawnCars
  (for _array_element (Variables|Default|GetLanes)
    (Game|SpawnActorfromClass "/Game/MyBP/Core/BP_Sedan.BP_Sedan_C" (Transformation|GetWorldTransform _array_element) "AlwaysSpawn" 0 0)))

(event EventSpawnPickups
  (bind _pickups (Variables|Default|GetPickups))
  (if (> (Utilities|Array|Length _pickups) 0)
    (Game|SpawnActorfromClass (Utilities|Array|Get(acopy) _pickups (Math|Random|RandomIntegerinRange 0 (Utilities|Array|LastIndex _pickups))) (Math|Transform|MakeTransform (Class|Tile|GetRandomPointinVolume) "0, 0, 0" "3.000000,3.000000,3.000000") "AlwaysSpawn" 0 0)
    (else
      (Development|PrintString "ERROR"))))

(fn ConstructionScript)